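; BP_Goal is a color-coded level exit that moves the player on to the next level.
; On BeginPlay it creates a dynamic material for its cylinder and tints it purple, blue or green from DefaultColor.
; When a BP_PlayerShawn overlaps the capsule with a matching current color, it increments the game instance's level index and calls LoadLevel.
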(event `self.ReceiveBeginPlay`
  (bind _mat (`self.Mat`))
  (bind _returnvalue (`KismetMaterialLibrary.CreateDynamicMaterialInstance` (`self.ParentMat`)))
  (bind _output_get (set `self.Mat` _returnvalue))
  (`PrimitiveComponent.SetMaterial` (`self.Cylinder`) 0 _output_get)
  (switch `/Game/BPShawn/E_ColorStock` (`self.DefaultColor`)
    (:`NewEnumerator0`
      (`MaterialInstanceDynamic.SetVectorParameterValue` _mat "Base Color" (struct :`R` 0.592157 :`G` 0.333333 :`B` 0.85098 :`A` 1.0)))
    (:`NewEnumerator1`
      (`MaterialInstanceDynamic.SetVectorParameterValue` _mat "Base Color" (struct :`R` 0.082353 :`G` 0.627451 :`B` 0.713726 :`A` 1.0)))
    (:`NewEnumerator2`
      (`MaterialInstanceDynamic.SetVectorParameterValue` _mat "Base Color" (struct :`R` 0.423529 :`G` 0.839216 :`B` 0.141176 :`A` 1.0)))))

(event `self.Capsule.OnComponentBeginOverlap`
  (params (OverlappedComponent :type "PrimitiveComponent Object Reference") (OtherActor :type "Actor Object Reference") (OtherComp :type "PrimitiveComponent Object Reference") (OtherBodyIndex :type Integer) (bFromSweep :type Boolean) (SweepResult :type "HitResult Structure (by ref)"))
  (bind _asbp_player_shawn (cast `/Game/BPShawn/BP_PlayerShawn` OtherActor))
  (if (`|EnumEquality` (`/Game/BPShawn/BP_PlayerShawn.CurrentColorE` _asbp_player_shawn) (`self.DefaultColor`))
    (bind _asbp_game_instance (cast `/Game/BPShawn/BP_GameInstance` (`GameplayStatics.GetGameInstance`)))
    (bind _result (`/Engine/EditorBlueprintResources/StandardMacros.IncrementInt` (`/Game/BPShawn/BP_GameInstance.CurrentLevelIndex` _asbp_game_instance))
      (:`  `
        (`/Game/BPShawn/BP_GameInstance.LoadLevel` _asbp_game_instance _result)))))

(fn `UserConstructionScript`)