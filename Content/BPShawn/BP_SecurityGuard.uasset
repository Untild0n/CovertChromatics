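; BP_SecurityGuard is a security guard child Blueprint that adds return-to-post behavior for guards flagged as static.
; At BeginPlay a static guard stores its starting transform.
; On Tick, any deviation from that transform leads through a WaitAfterChase delay to an AIMoveTo back to the start location, restoring the original rotation on success.
; An unconnected construction-script loop for showing sprite components never runs.
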(event `self.ReceiveBeginPlay`
  (`parent.ReceiveBeginPlay`)
  (if (`self.isStatic`)
    (set `self.StartTransform` (`self.GetTransform`))))

(event `self.ReceiveTick`
  (params (DeltaSeconds :type "Float (single-precision)"))
  (bind (_starttransform_location _starttransform_rotation) (`KismetMathLibrary.BreakTransform` (`self.StartTransform`)))
  (`parent.ReceiveTick` DeltaSeconds)
  (if (`self.isStatic`)
    (if (not (== (`self.StartTransform`) (`self.GetTransform`)))
      (`KismetSystemLibrary.Delay` (`self.WaitAfterChase`))
      (`|AIMoveTo` self _starttransform_location null 20.0
        (:`OnSuccess`
          (`self.K2_SetActorRotation` _starttransform_rotation))))))

(fn `UserConstructionScript`
  (`parent.UserConstructionScript`))