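; BP_SecurityManager is a manager that tracks which security units currently see the player and triggers game over on prolonged detection.
; PlayerSpotted and PlayerHiding events add and remove spotters from a list.
; While any remain, Tick drains a shared grace timer, reloading the level through BP_GameInstance below zero, and refills it after a reset delay unseen.
; Timeline start, resume and pause events exist, but no timeline outputs are wired.
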(event `self.ReceiveBeginPlay`
  (`KismetSystemLibrary.Delay` 0.2)
  (bind _returnvalue (`GameplayStatics.GetActorOfClass` "/Game/BPShawn/BP_PlayerShawn.BP_PlayerShawn_C"))
  (set `self.Player` _returnvalue))

(event `PlayerSpotted`
  (params (Security :type "/Game/BPShawn/BP_Security Object Reference"))
  (bind _securityspottingplayer (`self.SecuritySpottingPlayer`))
  (if (not (`KismetArrayLibrary.Array_Contains` _securityspottingplayer))
    (`KismetArrayLibrary.Array_Add` _securityspottingplayer Security)))

(event `PlayerHiding`
  (params (Security :type "/Game/BPShawn/BP_Security Object Reference"))
  (`KismetArrayLibrary.Array_RemoveItem` (`self.SecuritySpottingPlayer`) Security))

(event `self.ReceiveTick`
  (params (DeltaSeconds :type "Float (single-precision)"))
  (bind _output_get (set `self.PlayerSpottted` (`KismetArrayLibrary.Array_IsNotEmpty` (`self.SecuritySpottingPlayer`))))
  (if _output_get
    (set `self.LastTimeSpotted` (`KismetMathLibrary.Now`))
    (bind _output_get_2 (set `self.GraceTimerCurrent` (- (`self.GraceTimerCurrent`) DeltaSeconds)))
    (`/Engine/EditorBlueprintResources/StandardMacros.CompareFloat` _output_get_2
      (:`<`
        (`KismetSystemLibrary.PrintString` "GameOver")
        (bind _asbp_game_instance (cast `/Game/BPShawn/BP_GameInstance` (`GameplayStatics.GetGameInstance`)))
        (`/Game/BPShawn/BP_GameInstance.Reload Current Level` _asbp_game_instance)))
    (elif (>= (- (`KismetMathLibrary.Now`) (`self.LastTimeSpotted`)) (`self.GraceResetTime`))
      (set `self.GraceTimerCurrent` (`self.GraceTimerMax`)))))

(event `ResumeTimeline`
  (`Timeline|Timeline` :!label _label))

(event `StartTimeline`
  (goto _label :!via `PlayFromStart`))

(event `PauseTimeline`
  (goto _label :!via `Stop`))

(fn `UserConstructionScript`)