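; BP_Security is a security guard pawn that patrols, or stands static, and detects the player through AI Perception.
; Tick moves it along PatrolPoints using simple navigation, with a flying variant, per-point waits, and route reversal when not cyclic.
; Perception updates report spotted or hiding to BP_SecurityManager, pausing or resuming Tick.
; ChangeColor tints its dynamic material and spotlight together.
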(event `self.ReceiveBeginPlay`
  (if (not (`self.isStatic`))
    (set `self.CurrentTargetPoint` (`|GetArrayItem` (`self.PatrolPoints`))))
  (`KismetSystemLibrary.Delay` 0.2)
  (bind _returnvalue (`GameplayStatics.GetActorOfClass` "/Game/BPShawn/BP_SecurityManager.BP_SecurityManager_C"))
  (set `self.SecurityManager` _returnvalue)
  (bind _returnvalue_2 (`KismetMaterialLibrary.CreateDynamicMaterialInstance` (`self.SecurityMatParent`)))
  (bind _output_get (set `self.SecurityMat` _returnvalue_2))
  (`PrimitiveComponent.SetMaterial` (`self.Mesh`) 0 _output_get)
  (`self.ChangeColor` (struct :`R` 0.679824 :`G` 0.059842 :`B` 1.0 :`A` 1.0))
  (`LightComponent.SetIntensity` (`self.SpotLight`) (`self.LightIntensity`)))

(event `self.ReceiveTick`
  (params (DeltaSeconds :type "Float (single-precision)"))
  (bind (_returnvalue_x _returnvalue_y) (`KismetMathLibrary.BreakVector` (`self.K2_GetActorLocation`)))
  (bind _returnvalue (`self.GetController`))
  (bind _currenttargetpoint_targetlocation (break `/Game/BPShawn/BP_PatrolPoint` (`self.CurrentTargetPoint`)))
  (bind _currenttargetpoint_targetlocation_2 (break `/Game/BPShawn/BP_PatrolPoint` (`self.CurrentTargetPoint`)))
  (bind (_currenttargetpoint_targetlocation_3 _currenttargetpoint_waittime) (break `/Game/BPShawn/BP_PatrolPoint` (`self.CurrentTargetPoint`)))
  (bind (_returnvalue_x_2 _returnvalue_y_2) (`KismetMathLibrary.BreakVector` (`self.K2_GetActorLocation` _currenttargetpoint_targetlocation_2)))
  (bind (_returnvalue_x_3 _returnvalue_y_3) (`KismetMathLibrary.BreakVector` (`self.K2_GetActorLocation` _currenttargetpoint_targetlocation)))
  (if (`self.isStatic`)
    _
    (elif (`self.isWaiting`)
      _
      (elif (== (`KismetMathLibrary.MakeVector` _returnvalue_x _returnvalue_y) (`KismetMathLibrary.MakeVector` _returnvalue_x_2 _returnvalue_y_2) :`ErrorTolerance` 50.0)
        (if (> _currenttargetpoint_waittime 0.0)
          (`self.StartWaitTimer`))
        (`self.UpdateTargetLocation`)
        (elif (`self.isFlying`)
          (`AIBlueprintHelperLibrary.SimpleMoveToLocation` _returnvalue (`KismetMathLibrary.MakeVector` _returnvalue_x_3 _returnvalue_y_3))
          (else
            (`AIBlueprintHelperLibrary.SimpleMoveToActor` _returnvalue _currenttargetpoint_targetlocation)))))))

(event `StartWaitTimer`
  (bind (_currenttargetpoint_targetlocation _currenttargetpoint_waittime) (break `/Game/BPShawn/BP_PatrolPoint` (`self.CurrentTargetPoint`)))
  (`MovementComponent.StopMovementImmediately` (`self.CharacterMovement`))
  (set `self.isWaiting` true)
  (`KismetSystemLibrary.Delay` _currenttargetpoint_waittime)
  (set `self.isWaiting` false))

(event `self.AIPerception.OnTargetPerceptionUpdated`
  (params (Actor :type "Actor Object Reference") (Stimulus :type "AIStimulus Structure"))
  (bind _securitymanager (`self.SecurityManager`))
  (if Stimulus_bSuccessfullySensed
    (`/Game/BPShawn/BP_SecurityManager.PlayerSpotted` _securitymanager self)
    (`KismetSystemLibrary.PrintString` "Spotted!")
    (`self.SetActorTickEnabled` false)
    (else
      (`/Game/BPShawn/BP_SecurityManager.PlayerHiding` _securitymanager self)
      (`KismetSystemLibrary.PrintString` "Hiding")
      (`self.SetActorTickEnabled` true))))

(event `self.AIPerception.OnPerceptionUpdated`
  (params (UpdatedActors :type "Array of Actor Object Reference (by ref)")))

(fn `ChangeColor`
  (params (TargetColor :type "LinearColor Structure"))
  (bind _output_get (set `self.CurrentColor` TargetColor))
  (`MaterialInstanceDynamic.SetVectorParameterValue` (`self.SecurityMat`) "Base Color" _output_get)
  (`LightComponent.SetLightColor` (`self.SpotLight`) _output_get true))

(fn `UpdateTargetLocation`
  (bind _result (`/Engine/EditorBlueprintResources/StandardMacros.IncrementInt` (`KismetArrayLibrary.Array_Find` (`self.PatrolPoints`) (`self.CurrentTargetPoint`)))
    (:`  `
      (bind _output_get (set `self.NextTargetIndex` _result))
      (if (> _output_get (- (`KismetArrayLibrary.Array_Length` (`self.PatrolPoints`)) 1))
        (if (not (`self.isCyclic`))
          (`KismetArrayLibrary.Array_Reverse` (`self.PatrolPoints`)))
        (set `self.NextTargetIndex` -1)
        (`self.UpdateTargetLocation`)
        (else
          (set `self.CurrentTargetPoint` (`|GetArrayItem` (`self.PatrolPoints`) _output_get)))))))

(fn `UserConstructionScript`)