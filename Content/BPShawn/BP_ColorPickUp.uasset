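; BP_ColorPickUp is a collectible that adds purple, blue or green color stock to the player.
; The construction script creates a dynamic material on the mesh, applies the default color and enables custom depth with a stencil value.
; ChangeColor tints the material and point light to match and stores the current color.
; When a BP_PlayerShawn overlaps the pickup radius, it receives the color and amount, then the pickup destroys itself.
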(event `self.ReceiveBeginPlay`)

(event `self.PIckupRadius.OnComponentBeginOverlap`
  (params (OverlappedComponent :type "PrimitiveComponent Object Reference") (OtherActor :type "Actor Object Reference") (OtherComp :type "PrimitiveComponent Object Reference") (OtherBodyIndex :type Integer) (bFromSweep :type Boolean) (SweepResult :type "HitResult Structure (by ref)"))
  (bind _asbp_player_shawn (cast `/Game/BPShawn/BP_PlayerShawn` OtherActor))
  (`/Game/BPShawn/BP_PlayerShawn.Add Color Stock` _asbp_player_shawn (`self.CurrentColor`) (`self.Amount`))
  (`self.K2_DestroyActor`))

(fn `ChangeColor`
  (params (TargetColor :type "/Game/BPShawn/E_ColorStock Enum" :default "NewEnumerator0"))
  (bind _color3 (`self.Color3`))
  (bind _color2 (`self.Color2`))
  (bind _pointlight (`self.PointLight`))
  (bind _mat (`self.Mat`))
  (bind _color1 (`self.Color1`))
  (switch `/Game/BPShawn/E_ColorStock` TargetColor
    (:`NewEnumerator0`
      (`MaterialInstanceDynamic.SetVectorParameterValue` _mat "Base Color" _color1)
      (`LightComponent.SetLightColor` _pointlight _color1 true))
    (:`NewEnumerator1`
      (`MaterialInstanceDynamic.SetVectorParameterValue` _mat "Base Color" _color2)
      (`LightComponent.SetLightColor` _pointlight _color2 true))
    (:`NewEnumerator2`
      (`MaterialInstanceDynamic.SetVectorParameterValue` _mat "Base Color" _color3)
      (`LightComponent.SetLightColor` _pointlight _color3 true)))
  (set `self.CurrentColor` TargetColor))

(fn `UserConstructionScript`
  (bind _staticmesh (`self.StaticMesh`))
  (bind _returnvalue (`KismetMaterialLibrary.CreateDynamicMaterialInstance` (`self.MatParent`)))
  (bind _output_get (set `self.Mat` _returnvalue))
  (`PrimitiveComponent.SetMaterial` (`self.StaticMesh`) 0 _output_get)
  (`self.ChangeColor` (`self.DefaultColor`))
  (`PrimitiveComponent.SetRenderCustomDepth` _staticmesh true)
  (`PrimitiveComponent.SetCustomDepthStencilValue` _staticmesh 1))