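; Security drone Blueprint that detects the player through a sight cone unless the player's current color matches its own.
; On detection it reports to the SecurityManager, disables its tick and stops movement.
; When the player leaves the cone, a spotting drone reports hiding, waits out a post-chase delay, then re-enables tick.
; Tick and construction defer to the parent; cone color and material setup nodes are disconnected.
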(event `self.ReceiveBeginPlay`
  (`parent.ReceiveBeginPlay`))

(event `self.ReceiveTick`
  (params (DeltaSeconds :type "Float (single-precision)"))
  (`parent.ReceiveTick` DeltaSeconds))

(event `self.SightCone.OnComponentBeginOverlap`
  (params (OverlappedComponent :type "PrimitiveComponent Object Reference") (OtherActor :type "Actor Object Reference") (OtherComp :type "PrimitiveComponent Object Reference") (OtherBodyIndex :type Integer) (bFromSweep :type Boolean) (SweepResult :type "HitResult Structure (by ref)"))
  (bind _asbp_player_shawn (cast `/Game/BPShawn/BP_PlayerShawn` OtherActor))
  (if (not (`|EnumEquality` (`/Game/BPShawn/BP_PlayerShawn.CurrentColorE` _asbp_player_shawn) (`self.CurrentColorE`)))
    (`/Game/BPShawn/BP_SecurityManager.PlayerSpotted` (`self.SecurityManager`) self)
    (`KismetSystemLibrary.PrintString` "Spotted!")
    (`self.SetActorTickEnabled` false)
    (`MovementComponent.StopMovementImmediately` (`self.CharacterMovement`))))

(event `self.SightCone.OnComponentEndOverlap`
  (params (OverlappedComponent :type "PrimitiveComponent Object Reference") (OtherActor :type "Actor Object Reference") (OtherComp :type "PrimitiveComponent Object Reference") (OtherBodyIndex :type Integer))
  (if (`KismetArrayLibrary.Array_Contains` (`/Game/BPShawn/BP_SecurityManager.SecuritySpottingPlayer` (`self.SecurityManager`)) self)
    (cast `/Game/BPShawn/BP_PlayerShawn` OtherActor)
    (`/Game/BPShawn/BP_SecurityManager.PlayerHiding` (`self.SecurityManager`) self)
    (`KismetSystemLibrary.PrintString` "Hiding")
    (`KismetSystemLibrary.Delay` (`self.WaitAfterChase`))
    (`self.SetActorTickEnabled` true)))

(fn `UserConstructionScript`
  (`parent.UserConstructionScript`))