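; BP_SecurityCamera is a security camera actor that swivels between target points unless marked static.
; Each tick it interpolates its rotation toward the current target's location using RotationSpeed.
; Once nearly aligned, it starts a wait timer and updates the target, holding rotation while waiting.
; The construction script applies the security material and enables custom depth with a stencil value on the mesh.
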(event `self.ReceiveBeginPlay`
  (`parent.ReceiveBeginPlay`))

(event `self.ReceiveTick`
  (params (DeltaSeconds :type "Float (single-precision)"))
  (bind _returnvalue (`self.K2_GetActorRotation`))
  (bind _currenttargetpoint_targetlocation (break `/Game/BPShawn/BP_PatrolPoint` (`self.CurrentTargetPoint`)))
  (bind _returnvalue_2 (`KismetMathLibrary.FindLookAtRotation` (`self.K2_GetActorLocation`) (`self.K2_GetActorLocation` _currenttargetpoint_targetlocation)))
  (if (`self.isStatic`)
    _
    (elif (`self.isWaiting`)
      _
      (elif (== _returnvalue _returnvalue_2 :`ErrorTolerance` 10.0)
        (`self.StartWaitTimer`)
        (`self.UpdateTargetLocation`)
        (else
          (`self.K2_SetActorRotation` (`KismetMathLibrary.RInterpTo` _returnvalue _returnvalue_2 (`GameplayStatics.GetWorldDeltaSeconds`) (`self.RotationSpeed`))))))))

(fn `UserConstructionScript`
  (bind _staticmesh (`self.StaticMesh`))
  (`parent.UserConstructionScript`)
  (`PrimitiveComponent.SetMaterial` (`self.StaticMesh`) 0 (`self.SecurityMat`))
  (`PrimitiveComponent.SetRenderCustomDepth` _staticmesh true)
  (`PrimitiveComponent.SetCustomDepthStencilValue` _staticmesh 1))