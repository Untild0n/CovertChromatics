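; BP_Projectile is a colored projectile that recolors BP_Security and BP_ColorPickUp actors it overlaps.
; On hitbox overlap, it changes the target to its own color if the player's current color stock is above zero and the target's color differs.
; A successful change deducts one unit of that color from the player and destroys the projectile.
; Its construction script applies the projectile material and enables custom depth with a stencil value.
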(event `self.ReceiveBeginPlay`)

(event `self.Hitbox.OnComponentBeginOverlap`
  (params (OverlappedComponent :type "PrimitiveComponent Object Reference") (OtherActor :type "Actor Object Reference") (OtherComp :type "PrimitiveComponent Object Reference") (OtherBodyIndex :type Integer) (bFromSweep :type Boolean) (SweepResult :type "HitResult Structure (by ref)"))
  (`self.Change Target Color` OtherActor))

(fn `Change Target Color`
  (params (TargetActor :type "Actor Object Reference"))
  (bind _color (`self.Color`))
  (bind _currentcolorstock (`/Game/BPShawn/BP_PlayerShawn.CurrentColorStock` (`self.Player`)))
  (bind _asbp_security (cast `/Game/BPShawn/BP_Security` TargetActor)
    (:`then`
      (`/Engine/EditorBlueprintResources/StandardMacros.CompareInt` _currentcolorstock
        (:`>`
          (if (not (`|EnumEquality` (`/Game/BPShawn/BP_Security.CurrentColorE` _asbp_security) (`self.Color`)))
            (`/Game/BPShawn/BP_Security.ChangeColor` _asbp_security _color)
            (`/Game/BPShawn/BP_PlayerShawn.Add Color Stock` (`self.Player`) _color -1 :!label _label)
            (`self.K2_DestroyActor`)))))
    (:`CastFailed`
      (bind _asbp_color_pick_up (cast `/Game/BPShawn/BP_ColorPickUp` TargetActor))
      (`/Engine/EditorBlueprintResources/StandardMacros.CompareInt` _currentcolorstock
        (:`>`
          (if (not (`|EnumEquality` (`self.Color`) (`/Game/BPShawn/BP_ColorPickUp.CurrentColor` _asbp_color_pick_up)))
            (`/Game/BPShawn/BP_ColorPickUp.ChangeColor` _asbp_color_pick_up _color)
            (goto _label)))))))

(fn `UserConstructionScript`
  (bind _projectile (`self.Projectile`))
  (`PrimitiveComponent.SetMaterial` (`self.Projectile`) 0 (`self.ProjMat`))
  (`PrimitiveComponent.SetRenderCustomDepth` _projectile true)
  (`PrimitiveComponent.SetCustomDepthStencilValue` _projectile 1))