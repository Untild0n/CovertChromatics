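; BP_SequenceTrigger is a box trigger that plays a timed, one-shot dialogue sequence when BP_PlayerShawn walks into it.
; On overlap it disables player input and steps through the Dialogue lines in the HUD text box, using a Delay loop.
; At the end it hides the box, restores input, registers itself in BP_GameInstance's TriggeredSequences and destroys itself.
; The overlap checks that list before playing.
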(event `self.ReceiveBeginPlay`
  (bind _asbp_hud (cast `/Game/Blueprints/BP_HUD` (`PlayerController.GetHUD` (`GameplayStatics.GetPlayerController` 0))))
  (set `self.HUD` _asbp_hud)
  (bind _asbp_game_instance (cast `/Game/BPShawn/BP_GameInstance` (`GameplayStatics.GetGameInstance`)))
  (set `self.GameInstance` _asbp_game_instance))

(event `self.Box.OnComponentBeginOverlap`
  (params (OverlappedComponent :type "PrimitiveComponent Object Reference") (OtherActor :type "Actor Object Reference") (OtherComp :type "PrimitiveComponent Object Reference") (OtherBodyIndex :type Integer) (bFromSweep :type Boolean) (SweepResult :type "HitResult Structure (by ref)"))
  (bind _dialogueindex (`self.DialogueIndex`))
  (bind _hud (`self.HUD`))
  (bind _asbp_player_shawn (cast `/Game/BPShawn/BP_PlayerShawn` OtherActor))
  (if (not (`KismetArrayLibrary.Array_Contains` (`/Game/BPShawn/BP_GameInstance.TriggeredSequences` (`self.GameInstance`))))
    (`self.DisableInput` _asbp_player_shawn (`GameplayStatics.GetPlayerController` 0))
    (`/Game/Blueprints/BP_HUD.ShowTextBox` (`self.HUD`) (`|GetArrayItem` (`self.Dialogue`)))
    (`/Engine/EditorBlueprintResources/StandardMacros.IncrementInt` (`self.DialogueIndex`)
      (:`  `
        (`KismetSystemLibrary.Delay` (`self.WaitBetweenLines`))
        (if (== (`KismetArrayLibrary.Array_Length` (`self.Dialogue`)) _dialogueindex) :!label _label
          (`/Game/Blueprints/BP_HUD.HideTextBox` _hud)
          (set `self.hasTriggered` true)
          (`self.EnableInput` _asbp_player_shawn (`GameplayStatics.GetPlayerController` 0))
          (`/Game/BPShawn/BP_GameInstance.AddTriggeredSequence` (`self.GameInstance`) self)
          (`self.K2_DestroyActor`)
          (else
            (`/Game/Blueprints/BP_HUD.EditText` _hud (`|GetArrayItem` (`self.Dialogue`) _dialogueindex))
            (`KismetSystemLibrary.Delay` (`self.WaitBetweenLines`))
            (`/Engine/EditorBlueprintResources/StandardMacros.IncrementInt` _dialogueindex
              (:`  `
                (goto _label)))))))))

(fn `UserConstructionScript`)